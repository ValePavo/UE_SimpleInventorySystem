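; Inventory component that holds a fixed number of item slots, handles adding items and drops them back into the world as pickups.
; AddItem uses the first matching or empty slot, clamping merged stacks to the item's max and discarding overflow.
; RemoveItemFromSlot takes one unit and spawns a BP_ItemPickup with that item's mesh at a random horizontal offset around player 0.
; Changes broadcast the slot array through OnInventoryUpdated.
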(event `self.ReceiveBeginPlay`
  (for _ (range (`self.MaxSlots`))
    (`KismetArrayLibrary.Array_Add` (`self.Slots`) (make `/Game/InventorySystem/Blueprints/Struct_InventorySlot` null))))

(fn `AddItem`
  (params (NewItemData :type "/Game/InventorySystem/Blueprints/BP_ItemData Object Reference") (NewQuantity :type Integer))
  (bind _slots (`self.Slots`))
  (for (_array_element _array_index) (`self.Slots`)
    (bind (_itemdata _quantity) (break `/Game/InventorySystem/Blueprints/Struct_InventorySlot` _array_element))
    (if (== NewItemData _itemdata)
      (`KismetArrayLibrary.Array_Set` _slots _array_index (make `/Game/InventorySystem/Blueprints/Struct_InventorySlot` _itemdata (`KismetMathLibrary.Clamp` (+ _quantity NewQuantity) 0 (`/Game/InventorySystem/Blueprints/BP_ItemData.MaxStack` _itemdata))))
      (`self.OnInventoryUpdated` _slots :!label _label)
      (break)
      (elif (== _itemdata null)
        (`KismetArrayLibrary.Array_Set` _slots _array_index (make `/Game/InventorySystem/Blueprints/Struct_InventorySlot` NewItemData NewQuantity))
        (goto _label)))))

(fn `RemoveItemFromSlot`
  (params (SlotIndex :type Integer))
  (locals (NewLocalVar :type "/Game/InventorySystem/Blueprints/BP_ItemData Object Reference"))
  (bind _slots (`self.Slots`))
  (bind (_itemdata _quantity) (break `/Game/InventorySystem/Blueprints/Struct_InventorySlot` (`|GetArrayItem` (`self.Slots`) SlotIndex)))
  (bind _returnvalue (- _quantity 1))
  (bind _returnvalue_2 (`|SpawnActorFromClass` "/Game/InventorySystem/Blueprints/BP_ItemPickup.BP_ItemPickup_C" (`KismetMathLibrary.Conv_VectorToTransform` (+ (* (`KismetMathLibrary.RandomFloatInRange` 80.0 150.0) (`KismetMathLibrary.Normal` (`KismetMathLibrary.MakeVector` (.x (`KismetMathLibrary.RandomUnitVector`)) (.y (`KismetMathLibrary.RandomUnitVector`))))) (`Actor.K2_GetActorLocation` (`GameplayStatics.GetPlayerCharacter` 0)))) "Undefined" "MultiplyWithRoot" null _itemdata null))
  (bind _staticmesh (`/Game/InventorySystem/Blueprints/BP_ItemPickup.StaticMesh` _returnvalue_2))
  (`StaticMeshComponent.SetStaticMesh` _staticmesh (`/Game/InventorySystem/Blueprints/BP_ItemData.PickupMesh` _itemdata))
  (`SceneComponent.SetRelativeScale3D` _staticmesh (`/Game/InventorySystem/Blueprints/BP_ItemData.MeshScale` _itemdata))
  (if (<= _returnvalue 0)
    (`KismetArrayLibrary.Array_Set` _slots SlotIndex (make `/Game/InventorySystem/Blueprints/Struct_InventorySlot` null))
    (else
      (`KismetArrayLibrary.Array_Set` _slots SlotIndex (make `/Game/InventorySystem/Blueprints/Struct_InventorySlot` _itemdata _returnvalue))))
  (`self.OnInventoryUpdated` _slots))